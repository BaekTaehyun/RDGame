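; Debug measuring tool that draws actor pivot axes and the distance between two chosen actors, from both the construction script and Tick.
; ShowPivot draws colored forward, right and up lines on every actor of ActorType's class.
; CheckDistanceTwoActor draws the flattened connecting line and X/Y legs, labeling direct and per-axis distances through DrawText on three TextRenders.
; AlwaysOn redraws continuously with short-lived lines, while CheckPivot and CheckDistance act as self-resetting one-shot toggles.
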(event EventTick
  (params (DeltaSeconds :type Float%20%28single-precision%29))
  (CallFunction|ShowPivot)
  (CallFunction|CheckDistanceTwoActor))

(event EventBeginPlay)

(fn ConstructionScript
  (CallFunction|ShowPivot)
  (CallFunction|CheckDistanceTwoActor))

(fn ShowPivot
  (bind _actortype (Variables|CheckPivot|GetActorType))
  (bind _durationtemp (Variables|CheckPivot|GetDurationTemp))
  (bind _pivotsize (Variables|CheckPivot|GetPivotSize))
  (bind _thickness (Variables|CheckPivot|GetThickness))
  (bind _returnvalue (Utilities|GetClass _actortype))
  (Variables|Default|GetAlwaysOn
    (:then
      (if (Utilities|IsValidClass _returnvalue) :!label _label
        (bind _outactors (Actor|GetAllActorsOfClass _returnvalue))
        (for _array_element _outactors
          (Rendering|Debug|DrawDebugLine (Transformation|GetActorLocation _array_element) (+ (Transformation|GetActorLocation _array_element) (* (Transformation|GetActorForwardVector _array_element) _pivotsize)) "(R=1.000000,G=0.000000,B=0.000000,A=1.000000)" _durationtemp _thickness "Foreground")
          (Rendering|Debug|DrawDebugLine (Transformation|GetActorLocation _array_element) (+ (Transformation|GetActorLocation _array_element) (* (Transformation|GetActorRightVector _array_element) _pivotsize)) "(R=0.000000,G=1.000000,B=0.000000,A=1.000000)" _durationtemp _thickness "Foreground")
          (Rendering|Debug|DrawDebugLine (Transformation|GetActorLocation _array_element) (+ (Transformation|GetActorLocation _array_element) (* (Transformation|GetActorUpVector _array_element) _pivotsize)) "(R=0.000000,G=0.000000,B=1.000000,A=1.000000)" _durationtemp _thickness "Foreground"))))
    (:else
      (if (Variables|CheckPivot|GetCheckPivot)
        (Variables|CheckPivot|SetCheckPivot false)
        (goto _label)))))

(fn CheckDistanceTwoActor
  (bind _textrender0 (Variables|Default|GetTextRender0))
  (bind __height (Variables|Default|Get_height))
  (bind _firstactor (Variables|CheckDistance|GetFirstActor))
  (bind _secondactor (Variables|CheckDistance|GetSecondActor))
  (bind _thickness (Variables|CheckPivot|GetThickness))
  (bind _returnvalue (Transformation|GetActorLocation _secondactor))
  (bind _returnvalue_2 (Transformation|GetActorLocation _firstactor))
  (bind (_x _y) (Math|Vector|BreakVector _returnvalue))
  (bind (_x_2 _y_2) (Math|Vector|BreakVector _returnvalue_2))
  (bind _x_3 (Math|Vector|BreakVector _returnvalue))
  (bind (_x_4 _y_3) (Math|Vector|BreakVector _returnvalue_2))
  (bind (_x_5 _y_4) (Math|Vector|BreakVector _returnvalue))
  (bind (_x_6 _y_5) (Math|Vector|BreakVector _returnvalue_2))
  (bind _returnvalue_3 (Math|Vector|MakeVector _x_2 _y_2 2.0))
  (bind _returnvalue_4 (Math|Vector|MakeVector _x_3 _y_2 2.0))
  (bind _returnvalue_5 (Math|Vector|MakeVector _x_5 _y_3 __height))
  (bind _returnvalue_6 (Math|Vector|MakeVector _x_5 _y_4 __height))
  (Variables|CheckPivot|SetDurationTemp (Variables|Default|GetDuration))
  (Variables|Default|GetAlwaysOn
    (:then
      (Variables|CheckPivot|SetDurationTemp 0.1)
      (Rendering|SetVisibility _textrender0 true false)
      (Variables|CheckDistance|GetFirstActor :!label _label
        (:then
          (Variables|CheckDistance|GetSecondActor
            (:then
              (Rendering|Debug|DrawDebugLine _returnvalue_3 _returnvalue_4 "(R=1.000000,G=0.000000,B=0.000000,A=1.000000)" (Variables|CheckPivot|GetDurationTemp) _thickness "Foreground")
              (Rendering|Debug|DrawDebugLine _returnvalue_5 _returnvalue_6 "(R=0.000000,G=1.000000,B=0.000000,A=1.000000)" (Variables|CheckPivot|GetDurationTemp) _thickness "Foreground")
              (Rendering|Debug|DrawDebugPoint (Math|Vector|MakeVector _x_6 _y_5 __height) 1e+01 "(R=1.000000,G=1.000000,B=1.000000,A=1.000000)" (Variables|CheckPivot|GetDurationTemp) "Foreground")
              (Rendering|Debug|DrawDebugPoint (Math|Vector|MakeVector _x _y __height) 1e+01 "(R=1.000000,G=1.000000,B=1.000000,A=1.000000)" (Variables|CheckPivot|GetDurationTemp) "Foreground")
              (Rendering|Debug|DrawDebugLine (Math|Vector|MakeVector _x_4 _y_3 __height) (Math|Vector|MakeVector _x_5 _y_4 __height) "(R=1.000000,G=1.000000,B=1.000000,A=1.000000)" (Variables|CheckPivot|GetDurationTemp) _thickness "Foreground")
              (CallFunction|DrawText _returnvalue_2 _returnvalue (Variables|Default|GetTextRender0))
              (CallFunction|DrawText _returnvalue_3 _returnvalue_4 (Variables|Default|GetTextRender1))
              (CallFunction|DrawText _returnvalue_5 _returnvalue_6 (Variables|Default|GetTextRender2)))
            (:else)))
        (:else)))
    (:else
      (if (Variables|CheckDistance|GetCheckDistance)
        (Variables|CheckDistance|SetCheckDistance false)
        (Rendering|SetVisibility _textrender0 true false)
        (goto _label)
        (else
          (Rendering|SetVisibility _textrender0 false false))))))

(fn DrawText
  (params (Pos1 :type Vector) (Pos2 :type Vector) (TexRender :type Text%20Render%20Component%20Object%20Reference))
  (bind _returnvalue (+ Pos1 Pos2))
  (bind _returnvalue_2 (* _returnvalue 0.5))
  (bind (_x _y) (Math|Vector|BreakVector _returnvalue_2))
  (Transformation|SetWorldLocation TexRender (Math|Vector|MakeVector _x _y (* (Variables|Default|Get_height) 5.0)) false true)
  (Transformation|SetWorldScale3D TexRender (Math|Conversions|ToVector(Float) (Variables|CheckDistance|GetTextSize)))
  (Rendering|Components|TextRender|SetText TexRender (Utilities|Text|ToText(String) (Utilities|String|ToString(Float) (Math|Vector|Distance(Vector) Pos1 Pos2)))))