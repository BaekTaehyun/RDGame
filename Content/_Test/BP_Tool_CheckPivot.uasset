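; Debug tool actor that visualizes the pivot location and orientation of every actor sharing the class of ActorType.
; CheckPivot acts as a one-shot button, polled by the construction script and Tick, that resets itself before drawing.
; Each actor gets foreground debug lines for forward (red), up (green) and right (blue), with configurable size, thickness and duration.
; Green and blue are swapped relative to Unreal's usual axis colors.
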(event EventTick
  (params (DeltaSeconds :type Float%20%28single-precision%29))
  (CallFunction|DrawDebugLine))

(fn ConstructionScript
  (CallFunction|DrawDebugLine))

(fn DrawDebugLine
  (bind _actortype (Variables|Default|GetActorType))
  (bind _duration (Variables|Default|GetDuration))
  (bind _pivotsize (Variables|Default|GetPivotSize))
  (bind _thickness (Variables|Default|GetThickness))
  (bind _returnvalue (Utilities|GetClass _actortype))
  (if (Variables|Default|GetCheckPivot)
    (Variables|Default|SetCheckPivot false)
    (if (Utilities|IsValidClass _returnvalue)
      (bind _outactors (Actor|GetAllActorsOfClass _returnvalue))
      (for _array_element _outactors
        (Rendering|Debug|DrawDebugLine (Transformation|GetActorLocation _array_element) (+ (Transformation|GetActorLocation _array_element) (* (Transformation|GetActorForwardVector _array_element) _pivotsize)) "(R=1.000000,G=0.000000,B=0.000000,A=1.000000)" _duration _thickness "Foreground")
        (Rendering|Debug|DrawDebugLine (Transformation|GetActorLocation _array_element) (+ (Transformation|GetActorLocation _array_element) (* (Transformation|GetActorUpVector _array_element) _pivotsize)) "(R=0.000000,G=1.000000,B=0.000000,A=1.000000)" _duration _thickness "Foreground")
        (Rendering|Debug|DrawDebugLine (Transformation|GetActorLocation _array_element) (+ (Transformation|GetActorLocation _array_element) (* (Transformation|GetActorRightVector _array_element) _pivotsize)) "(R=0.000000,G=0.000000,B=1.000000,A=1.000000)" _duration _thickness "Foreground")))))